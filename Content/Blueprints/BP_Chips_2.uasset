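; BP_Chips_2 is a moving pawn that destroys any BP_Bikerguy_Base actor it overlaps.
; Every Tick it feeds movement input along world negative X, so it travels in one fixed direction.
; An unconnected chain that would add Chips to CurrentPoints on BP_GameMode_Base never runs, so overlapping awards no points.
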(event `self.ReceiveActorBeginOverlap`
  (params (OtherActor :type "Actor Object Reference"))
  (bind _asbp_bikerguy_base (cast `/Game/Blueprints/BP_Bikerguy_Base` OtherActor))
  (`self.K2_DestroyActor` _asbp_bikerguy_base))

(event `self.ReceiveTick`
  (params (DeltaSeconds :type "Float (single-precision)"))
  (`self.AddMovementInput` (-1.0 0.0 0.0)))

(fn `UserConstructionScript`)